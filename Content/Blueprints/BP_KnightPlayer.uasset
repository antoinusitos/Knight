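; BP_KnightPlayer is the knight player Blueprint, which sets up its HUD and weapon when play begins.
; It creates the UMG_HUD widget, adds it to the viewport and initializes the UMGStats6 sub-widget with itself.
; It then spawns BP_Blade_BlackKnight, snaps it to the RightHandSocket on its mesh and stores it as TheWeapon.
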(event EventBeginPlay
  (Utilities|FlowControl|Sequence
    (:then_0
      (bind _returnvalue (UserInterface|CreateWidget "/Game/UMG/UMG_HUD.UMG_HUD_C"))
      (bind _output_get (Variables|Default|SetHUD _returnvalue))
      (UserInterface|Viewport|AddtoViewport _output_get 0)
      (Default|Init (Variables|/Game/UMG/UMG_HUD.UMG_HUD_C|GetUMG_Stats_6 _output_get) self))
    (:then_1
      (bind _returnvalue_2 (Game|SpawnActorfromClass "/Game/Blueprints/BP_Blade_BlackKnight.BP_Blade_BlackKnight_C" (Transformation|GetActorTransform) "Undefined" 0 0))
      (Transformation|AttachComponentToComponent _returnvalue_2 (Variables|Character|GetMesh) "RightHandSocket" "SnapToTarget" "SnapToTarget" "SnapToTarget" true)
      (Variables|Default|Set_theWeapon _returnvalue_2))))

(fn ConstructionScript)